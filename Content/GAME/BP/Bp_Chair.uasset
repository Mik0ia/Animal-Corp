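; Chair actor that seats the first-person player character when interacted with.
; Activation of its interactable component, if the character is on the ground, zeroes velocity and disables the character's collision.
; It then snaps the capsule slightly above the Box position, aligned to the Arrow's rotation, and sets IsSit on the character.
; The QuitChair event is empty, so this Blueprint contains no stand-up logic.
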(event OnComponentActivated(BPC_Iinteractable)
  (params (Component :type Actor%20Component%20Object%20Reference) (bReset :type Boolean))
  (bind _bpc_iinteractable (Variables|Default|GetBPC_Iinteractable))
  (bind _box (Variables|Default|GetBox))
  (bind _returnvalue (Transformation|GetWorldLocation _box))
  (bind _as_bp_first_person_character (Variables|/Game/GAME/BP/BPC/BPC_Iinteractable.BPC_Iinteractable_C|GetAs%20BP%20First%20Person%20Character _bpc_iinteractable))
  (bind _charactermovement (Variables|/Script/Engine.Character|GetCharacterMovement _as_bp_first_person_character))
  (if (AI|Components|NavMovement|IsMovingonGround _charactermovement)
    (Variables|/Script/Engine.MovementComponent|SetVelocity _charactermovement "0, 0, 0")
    (Collision|SetActorEnableCollision _as_bp_first_person_character false)
    (Transformation|SetWorldLocationAndRotation (Variables|/Script/Engine.Character|GetCapsuleComponent _as_bp_first_person_character) (Math|Vector|MakeVector (.x _returnvalue) (.y _returnvalue) (+ (.z _returnvalue) 25.0)) (Transformation|GetWorldRotation (Variables|Default|GetArrow)) false false)
    (Variables|/Game/GAME/BP/BP_FirstPersonCharacter.BP_FirstPersonCharacter_C|SetIs%20Sit%20? _as_bp_first_person_character true)))

(event Custom|Quit%20Chair)

(event EventBeginPlay)

(event Collision|EventActorBeginOverlap
  (params (OtherActor :type Actor%20Object%20Reference)))

(event EventTick
  (params (DeltaSeconds :type Float%20%28single-precision%29)))

(fn ConstructionScript)