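; BPC_Dialoguable is a component that handles the start of a dialogue, presumably on the actor that owns it.
; StartDialogue turns SMRotation toward the player's first-person camera, using a look-at rotation with pitch zeroed so it stays upright.
; It then makes the referenced dialogue widget component visible.
; The graph does not set the references it uses or handle ending the dialogue.
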(event Custom|StartDialogue
  (bind _sm_rotation (Variables|Default|GetSM_Rotation))
  (bind _playerref (Variables|Default|GetPlayerRef))
  (bind _returnvalue (Transformation|GetWorldLocation _sm_rotation))
  (bind _firstpersoncamera (Variables|/Game/GAME/BP/BP_FirstPersonCharacter.BP_FirstPersonCharacter_C|GetFirstPersonCamera _playerref))
  (bind _returnvalue_2 (Transformation|GetWorldLocation _firstpersoncamera))
  (bind _returnvalue_3 (- _returnvalue_2 _returnvalue))
  (bind _returnvalue_4 (Math|Rotator|MakeRotfromX _returnvalue_3))
  (Transformation|SetWorldRotation (Variables|Default|GetSM_Rotation) (Math|Rotator|MakeRotator (.roll _returnvalue_4) 0.0 (.yaw _returnvalue_4)) false false)
  (Rendering|SetVisibility (Variables|Default|GetDialogue%20Widget%20Ref) true false))