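; Test character for the dialogue system that wanders in random directions and carries a BPCDialoguable component.
; Construction applies the configured skeletal mesh, hands the component its owner and capsule, and seeds the walk direction from the capsule's forward vector.
; Unless immobile or barred from walking, Tick adds movement input along that direction and calls Rotate, which picks a new normalized random vector, then uses a flag and random delay to space out changes.
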(event Custom|Rotate
  (if (not (Variables|Default|GetIs%20rotating?))
    (Variables|Default|SetIs%20rotating? true)
    (Variables|Default|SetRotation%20Vector (Math|Vector|Normalize (Utilities|RandomVector (Variables|Collision|GetCapsuleComponent))))
    (Utilities|FlowControl|Delay (Math|Random|RandomFloatinRange 5.0 1e+01))
    (Variables|Default|SetIs%20rotating? false)))

(event EventBeginPlay)

(event Collision|EventActorBeginOverlap
  (params (OtherActor :type Actor%20Object%20Reference)))

(event EventTick
  (params (DeltaSeconds :type Float%20%28single-precision%29))
  (if (not (Variables|Default|GetImmobile%20?))
    (if (Variables|Default|GetCan%20Walk%20?)
      (Pawn|Input|AddMovementInput (Variables|Default|GetRotation%20Vector) 1.0 false)
      (CallFunction|Rotate))))

(fn ConstructionScript
  (bind _bpc_dialoguable (Variables|Default|GetBPC_Dialoguable))
  (Components|SkeletalMesh|SetSkeletalMeshAsset (Variables|Character|GetMesh) (Variables|Default|GetSkm))
  (Variables|/Game/GAME/BP/BPC/BPC_Dialoguable.BPC_Dialoguable_C|SetOwnerRef _bpc_dialoguable self)
  (Variables|/Game/GAME/BP/BPC/BPC_Dialoguable.BPC_Dialoguable_C|SetSM_Rotation _bpc_dialoguable (Variables|Collision|GetCapsuleComponent))
  (Variables|Default|SetRotation%20Vector (Math|Vector|GetForwardVector (Variables|Collision|GetCapsuleComponent))))