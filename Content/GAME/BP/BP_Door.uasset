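; Interactable door Blueprint that swings open or closed when its BPC_Iinteractable component is activated.
; An IsOpen flag selects between two timelines, one played forward to open and the other reversed from its end to close, each driving the mesh's relative yaw.
; IsMoving blocks retriggering mid-swing, while mesh collision is switched off during motion and restored when the timeline finishes.
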(event OnComponentActivated(BPC_Iinteractable)
  (params (Component :type Actor%20Component%20Object%20Reference) (bReset :type Boolean))
  (bind _staticmesh (Variables|Default|GetStaticMesh))
  (bind _staticmesh_2 (Variables|Default|GetStaticMesh))
  (if (not (Variables|Default|GetIs%20moving%20?))
    (Variables|Default|SetIs%20moving%20? true)
    (if (Variables|Default|GetIs%20open%20?)
      (Variables|Default|SetIs%20open%20? false)
      (bind _output_get (Variables|Default|SetCollision (Collision|GetCollisionEnabled _staticmesh_2)))
      (Collision|SetCollisionEnabled _staticmesh_2 "NoCollision")
      (bind _newtrack_0 (Timeline|Timeline_0 ReverseFromEnd)
        (:Update
          (Transformation|SetRelativeRotation (Variables|Default|GetStaticMesh) (Math|Rotator|MakeRotator 0.0 0.0 _newtrack_0) false false))
        (:Finished
          (Variables|Default|SetIs%20moving%20? false)
          (Collision|SetCollisionEnabled _staticmesh _output_get)))
      (else
        (Variables|Default|SetIs%20open%20? true)
        (bind _output_get_2 (Variables|Default|SetCollision (Collision|GetCollisionEnabled _staticmesh)))
        (Collision|SetCollisionEnabled _staticmesh "NoCollision")
        (bind _newtrack_0_2 (Timeline|Timeline PlayFromStart)
          (:Update
            (Transformation|SetRelativeRotation _staticmesh_2 (Math|Rotator|MakeRotator 0.0 0.0 _newtrack_0_2) false false))
          (:Finished
            (Variables|Default|SetIs%20moving%20? false)
            (Collision|SetCollisionEnabled _staticmesh _output_get_2)))))))

(event EventBeginPlay)

(event Collision|EventActorBeginOverlap
  (params (OtherActor :type Actor%20Object%20Reference)))

(fn ConstructionScript)